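; Player camera manager for the toon character that supplies camera tuning for each movement state.
; GetCameraParamet selects rotation lag and pivot height by rotation mode, then nests Stance and Gait switches to choose camera offsets and per-axis pivot lag speeds.
; SetCameraParamet writes those values to variables, while BlueprintUpdateCamera only passes through the parent's result.
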(event `self.GetCameraParamet`
  (bind _stance (`self.Stance`))
  (bind _gait (`self.Gait`))
  (switch `ERotationMode` (`self.RotationMode`)
    (:`VelocityDirection`
      (set `self.RotationLagSpeed` 20.0)
      (switch `EStance` _stance
        (:`Standing`
          (set `self.PivotOffset_Z` 50.0)
          (switch `EGait` _gait
            (:`Walking`
              (`self.SetCameraParamet` -325.0 0.0 50.0 5.0 5.0 15.0))
            (:`Running`
              (`self.SetCameraParamet` -325.0 0.0 20.0 5.0 5.0 15.0))
            (:`Sprinting`
              (`self.SetCameraParamet` -325.0 0.0 20.0 5.0 5.0 15.0))))))
    (:`LookingDirection`
      (set `self.RotationLagSpeed` 20.0)
      (switch `EStance` _stance
        (:`Standing`
          (set `self.PivotOffset_Z` 40.0)
          (switch `EGait` _gait
            (:`Walking`
              (`self.SetCameraParamet` -275.0 75.0 35.0 8.0 8.0 15.0))
            (:`Running`
              (`self.SetCameraParamet` -275.0 75.0 35.0 4.0 6.0 15.0))
            (:`Sprinting`
              (`self.SetCameraParamet` -250.0 70.0 5.0 10.0 5.0 15.0))))))
    (:`Aiming`
      (set `self.RotationLagSpeed` 20.0)
      (switch `EStance` _stance
        (:`Standing`
          (set `self.PivotOffset_Z` 50.0)
          (switch `EGait` _gait
            (:`Walking`
              (`self.SetCameraParamet` -200.0 70.0 35.0 15.0 15.0 15.0))
            (:`Running`
              (`self.SetCameraParamet` -200.0 70.0 35.0 15.0 15.0 15.0))
            (:`Sprinting`
              (`self.SetCameraParamet` -200.0 70.0 5.0 10.0 5.0 15.0))))))))

(fn `BlueprintUpdateCamera`
  (params (CameraTarget :type "Actor Object Reference"))
  (returns (NewCameraLocation :type "Vector Structure") (NewCameraRotation :type "Rotator Structure") (NewCameraFOV :type "Float (single-precision)") (ReturnValue :type Boolean))
  (bind (_newcameralocation _newcamerarotation _newcamerafov _returnvalue) (`parent.BlueprintUpdateCamera` CameraTarget))
  (return _newcameralocation _newcamerarotation _newcamerafov _returnvalue))

(fn `SetCameraParamet`
  (params (`Camera Offset X` :type "Float (single-precision)") (`Camera Offset Y` :type "Float (single-precision)") (`Camera Offset Z` :type "Float (single-precision)") (`Pivot Lag Speed X` :type "Float (single-precision)") (`Pivot Lag Speed Y` :type "Float (single-precision)") (`Pivot Lag Speed Z` :type "Float (single-precision)"))
  (set `self.CameraOffset_X` `Camera Offset X`)
  (set `self.CameraOffset_Y` `Camera Offset Y`)
  (set `self.CameraOffset_Z` `Camera Offset Z`)
  (set `self.PivotLagSpeed_X` `Pivot Lag Speed X`)
  (set `self.PivotLagSpeed_Y` `Pivot Lag Speed Y`)
  (set `self.PivotLagSpeed_Z` `Pivot Lag Speed Z`))

(fn `UserConstructionScript`)